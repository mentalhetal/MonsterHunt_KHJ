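; BP_Paladin is the player's melee character, with camera-relative movement, sprint, two-hit combo, shield block, dodge roll and death screen.
; State booleans gate Enhanced Input actions, which are bound by a custom Input event along with the HUD widget.
; Externally triggered events chain combos and apply sphere-trace damage, while blocking reduces and rolling negates incoming damage.
; Actions spend stamina, timelines handle continuous drain and idle recovery, and health and stamina feed HUD bars.
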(event Custom|AttackCheck
  (bind _returnvalue (Transformation|GetActorLocation))
  (bind _returnvalue_2 (Transformation|GetActorForwardVector))
  (bind _fwdlocation (Variables|공격|GetFwdLocation))
  (bind _spawntransformlocation (Variables|공격|GetSpawnTransformLocation))
  (bind _returnvalue_3 (* _returnvalue_2 _fwdlocation))
  (bind _returnvalue_4 (+ _returnvalue _returnvalue_3))
  (bind _returnvalue_5 (+ _returnvalue_4 _spawntransformlocation))
  ;[1 1 1] 공격 체크
  (bind (_outhit _returnvalue_6) (Class|KismetSystemLibrary|SphereTraceSinglebyProfile _returnvalue_5 _returnvalue_5 1e+02 "MonsterBody" false 0 "None" true "(R=1.000000,G=0.000000,B=0.000000,A=1.000000)" "(R=0.000000,G=1.000000,B=0.000000,A=1.000000)" 0.5))
  (Game|Damage|ApplyPointDamage (.HitActor (Collision|BreakHitResult _outhit)) (Variables|공격|GetPlayerDamege) (.ImpactPoint (Collision|BreakHitResult _outhit)) _outhit 0 self "/Engine/EngineDamageTypes/DmgTypeBP_Environmental.DmgTypeBP_Environmental_C"))

(event Custom|ResetAttack
  ;[1 1 1] 공격 초기화
  (Variables|공격|SetIsAttack false)
  (Variables|공격|SetComboCount 0)
  (Variables|공격|SetIsComboAttack false)
  (Variables|회피|SetIsRoll false))

(event Custom|HPUpdate
  (bind _curhp (Variables|체력|GetCurHP))
  (bind _ascharacter_ui (Utilities|Casting|CastToCharacterUI (Variables|Default|GetCharacterUI)))
  (Default|SetPBHPPersent _ascharacter_ui (/ _curhp (Variables|체력|GetmaxHP)))
  (if (<= _curhp 0.0)
    (Variables|체력|SetIsDie true)
    (CallFunction|Death)))

(event Custom|ComboAction
  ;[1 1 1] 마우스 왼쪽 클릭 - 공격
  (if (not (Math|Boolean|ORBoolean (Variables|체력|GetIsDie) (Variables|회피|GetIsRoll) (Variables|Default|GetIsBlock)))
    (if (Variables|공격|GetIsComboAttack)
      (Variables|공격|SetIsComboAttack false)
      (bind (_attackable _curst) (CallFunction|AttackSpentST))
      (if _attackable
        (switch int (Variables|공격|GetComboCount)
          (:0
            (Animation|Montage|PlayMontage (Variables|Character|GetMesh) "/Game/02_Resource/Anim/Paladin/AM_Paladin_Attack_A.AM_Paladin_Attack_A" 1.5
              (:then
                (Math|Integer|IncrementInt (Variables|공격|GetComboCount)
                  (:%20%20
                    _)))))
          (:1
            (Animation|Montage|PlayMontage (Variables|Character|GetMesh) "/Game/02_Resource/Anim/Paladin/AM_Paladin_Attack_B.AM_Paladin_Attack_B" 1.5
              (:then
                _))))
        (else
          (CallFunction|ResetAttack)))
      (Variables|스테미나|SetCurST _curst)
      (CallFunction|SteminaUpdate))))

(event Custom|Death
  (Utilities|FlowControl|DoOnce false
    (:Completed
      (bind _returnvalue (UserInterface|CreateWidget "/Game/01_BluePrint/03_UI/DeathUI.DeathUI_C"))
      (UserInterface|Viewport|AddtoViewport _returnvalue 0)
      (Components|Animation|PlayAnimation (Variables|Character|GetMesh) "/Game/02_Resource/Anim/Paladin/Paladin_Death.Paladin_Death" false))))

(event Custom|SteminaUpdate
  (bind _ascharacter_ui (Utilities|Casting|CastToCharacterUI (Variables|Default|GetCharacterUI)))
  (Default|SetPBSTPersent _ascharacter_ui (/ (Variables|스테미나|GetCurST) (Variables|스테미나|GetMaxST))))

(event Custom|Input
  ;[1 1 1] 인트로 동영상 끝나고 Input 받기용
  (bind _as플레이어_컨트롤러 (Utilities|Casting|CastToPlayerController (Pawn|GetController)))
  (Utilities|IsValid _as플레이어_컨트롤러
    (:Is%20Valid
      (Input|AddMappingContext (PlayerController|LocalPlayerSubsystems|GetEnhancedInputLocalPlayerSubsystem _as플레이어_컨트롤러) "/Game/01_BluePrint/00_Global/Input/IM_Context.IM_Context" 0 "(bIgnoreAllPressedKeysUntilRelease=True,bForceImmediately=False,bNotifyUserSettings=False)")
      (bind _asbp_hud (Utilities|Casting|CastToBP_HUD (HUD|GetHUD _as플레이어_컨트롤러)))
      (Variables|Default|SetCharacterUI (Variables|/Game/01_BluePrint/02_Frame/BP_HUD.BP_HUD_C|GetCharacterUI _asbp_hud))
      (CallFunction|HPUpdate)
      (CallFunction|SteminaUpdate))))

(event Custom|ResetRoll
  ;[1 1 1] 회피 초기화
  (Variables|회피|SetIsRoll false)
  (Variables|공격|SetIsAttack false)
  (Variables|공격|SetComboCount 0)
  (Variables|공격|SetIsComboAttack false))

(event Custom|SlashSound
  (bind _returnvalue (Transformation|GetActorLocation))
  (bind _returnvalue_2 (Transformation|GetActorForwardVector))
  (bind _fwdlocation (Variables|공격|GetFwdLocation))
  (bind _spawntransformlocation (Variables|공격|GetSpawnTransformLocation))
  (bind _returnvalue_3 (* _returnvalue_2 _fwdlocation))
  (bind _returnvalue_4 (+ _returnvalue _returnvalue_3))
  (bind _returnvalue_5 (+ _returnvalue_4 _spawntransformlocation))
  ;[1 1 1] 칼 휘두를때 소리
  (if (stale Custom|AttackCheck _returnvalue_6)
    (if (== (Variables|공격|GetComboCount) 0)
      (Audio|PlaySoundatLocation "/Game/02_Resource/Sound/Paladin/SQ_Paladin_HitSlash_01.SQ_Paladin_HitSlash_01" _returnvalue_5 "0, 0, 0" 1.0 1.0 0.0 0 0 0 0)
      (else
        (Audio|PlaySoundatLocation "/Game/02_Resource/Sound/Paladin/SQ_Paladin_HitSlash_02.SQ_Paladin_HitSlash_02" _returnvalue_5 "0, 0, 0" 1.0 1.0 0.0 0 0 0 0)))
    (else
      (Audio|PlaySoundatLocation "/Game/02_Resource/Sound/Paladin/SQ_Paladin_Slash_01.SQ_Paladin_Slash_01" _returnvalue_5 "0, 0, 0" 1.0 1.0 0.0 0 0 0 0))))

(event Custom|ShieldSound
  (Audio|PlaySoundatLocation "/Game/02_Resource/Sound/Paladin/SQ_Paladin_Shield.SQ_Paladin_Shield" (Transformation|GetSocketLocation (Variables|Character|GetMesh) "Shield_joint") "0, 0, 0" 1.0 1.0 0.0 0 0 0 0))

(event Input|EnhancedActionEvents|EnhancedInputActionIA_MoveForward
  (params (ActionValue :type Float%20%28double-precision%29) (ElapsedSeconds :type Float%20%28double-precision%29) (TriggeredSeconds :type Float%20%28double-precision%29) (InputAction :type Input%20Action%20Object%20Reference :default "/Game/01_BluePrint/00_Global/Input/IA_MoveForward.IA_MoveForward"))
  (if (not (Math|Boolean|ORBoolean (Variables|체력|GetIsDie) (Variables|공격|GetIsAttack) (Variables|회피|GetIsRoll) (Variables|Default|GetIsBlock)))
    (Pawn|Input|AddMovementInput (Math|Vector|GetForwardVector (Math|Rotator|MakeRotator 0.0 0.0 (.yaw (Pawn|GetControlRotation :!class /Script/Engine.Pawn)))) ActionValue false)))

(event Input|EnhancedActionEvents|EnhancedInputActionIA_MoveRight
  (params (ActionValue :type Float%20%28double-precision%29) (ElapsedSeconds :type Float%20%28double-precision%29) (TriggeredSeconds :type Float%20%28double-precision%29) (InputAction :type Input%20Action%20Object%20Reference :default "/Game/01_BluePrint/00_Global/Input/IA_MoveRight.IA_MoveRight"))
  (if (not (Math|Boolean|ORBoolean (Variables|체력|GetIsDie) (Variables|공격|GetIsAttack) (Variables|회피|GetIsRoll) (Variables|Default|GetIsBlock)))
    (Pawn|Input|AddMovementInput (Math|Vector|GetRightVector (Math|Rotator|MakeRotator 0.0 0.0 (.yaw (Pawn|GetControlRotation :!class /Script/Engine.Pawn)))) ActionValue false)))

(event Input|EnhancedActionEvents|EnhancedInputActionIA_MouseXY
  (params (ActionValue :type Vector%202D%20Structure) (ElapsedSeconds :type Float%20%28double-precision%29) (TriggeredSeconds :type Float%20%28double-precision%29) (InputAction :type Input%20Action%20Object%20Reference :default "/Game/01_BluePrint/00_Global/Input/IA_MouseXY.IA_MouseXY"))
  ;[1 1 1] 마우스 상하좌우 카메라 이동
  (if (not (Variables|체력|GetIsDie))
    (Pawn|Input|AddControllerYawInput (.x ActionValue))
    (Pawn|Input|AddControllerPitchInput (.y ActionValue))))

(event Input|EnhancedActionEvents|EnhancedInputActionIA_MouseLeftClick
  (params (ActionValue :type Boolean) (ElapsedSeconds :type Float%20%28double-precision%29) (TriggeredSeconds :type Float%20%28double-precision%29) (InputAction :type Input%20Action%20Object%20Reference :default "/Game/01_BluePrint/00_Global/Input/IA_MouseLeftClick.IA_MouseLeftClick"))
  ;[1 1 1] 마우스 왼쪽 클릭 - 공격
  (:Started
    (if (not (Math|Boolean|ORBoolean (Variables|체력|GetIsDie) (Variables|회피|GetIsRoll) (Variables|Default|GetIsBlock)))
      (if (Variables|공격|GetIsAttack)
        (Variables|공격|SetIsComboAttack true)
        (else
          (Variables|공격|SetIsAttack true)
          (bind (_attackable _curst) (CallFunction|AttackSpentST))
          (if _attackable
            (switch int (Variables|공격|GetComboCount)
              (:0
                (Animation|Montage|PlayMontage (Variables|Character|GetMesh) "/Game/02_Resource/Anim/Paladin/AM_Paladin_Attack_A.AM_Paladin_Attack_A" 1.5
                  (:then
                    (Math|Integer|IncrementInt (Variables|공격|GetComboCount)
                      (:%20%20
                        _)))))
              (:1
                (Animation|Montage|PlayMontage (Variables|Character|GetMesh) "/Game/02_Resource/Anim/Paladin/AM_Paladin_Attack_B.AM_Paladin_Attack_B" 1.5
                  (:then
                    _))))
            (else
              (CallFunction|ResetAttack)))
          (Variables|스테미나|SetCurST _curst)
          (CallFunction|SteminaUpdate))))))

(event Input|EnhancedActionEvents|EnhancedInputActionIA_SwitchCamera
  (params (ActionValue :type Boolean) (ElapsedSeconds :type Float%20%28double-precision%29) (TriggeredSeconds :type Float%20%28double-precision%29) (InputAction :type Input%20Action%20Object%20Reference :default "/Game/01_BluePrint/00_Global/Input/IA_SwitchCamera.IA_SwitchCamera"))
  ;[1 1 1] 보류
  (:Started
    (if (Variables|Default|GetIsTabDown)
      (Variables|Default|SetIsTabDown false)
      (else
        (Variables|Default|SetIsTabDown true)))))

(event Input|EnhancedActionEvents|EnhancedInputActionIA_LeftShiftDown
  (params (ActionValue :type Boolean) (ElapsedSeconds :type Float%20%28double-precision%29) (TriggeredSeconds :type Float%20%28double-precision%29) (InputAction :type Input%20Action%20Object%20Reference :default "/Game/01_BluePrint/00_Global/Input/IA_LeftShiftDown.IA_LeftShiftDown"))
  (bind _charactermovement (Variables|Character|GetCharacterMovement))
  (bind _mesh (Variables|Character|GetMesh))
  (bind _returnvalue (Components|SkeletalMesh|GetAnimInstance _mesh))
  (:Triggered
    (if (not (Math|Boolean|ORBoolean (Variables|공격|GetIsAttack) (Variables|체력|GetIsDie) (Variables|회피|GetIsRoll) (Variables|Default|GetIsBlock))) :!label _label
      (if ActionValue
        (bind _asabp_paladin (Utilities|Casting|CastToABP_Paladin _returnvalue))
        (Variables|/Game/01_BluePrint/01_Character/ABP_Paladin.ABP_Paladin_C|SetIsShiftDown _asabp_paladin true)
        (bind _userunst (Timeline|타임라인_UseRunST Play)
          (:Update
            (Variables|스테미나|SetCurST (- (Variables|스테미나|GetCurST) _userunst))
            (CallFunction|SteminaUpdate)
            (Variables|/Script/Engine.CharacterMovementComponent|SetMaxWalkSpeed _charactermovement 7e+02)))
        (else
          (bind _asabp_paladin_2 (Utilities|Casting|CastToABP_Paladin _returnvalue))
          (Variables|/Game/01_BluePrint/01_Character/ABP_Paladin.ABP_Paladin_C|SetIsShiftDown _asabp_paladin_2 false)
          (CallFunction|SteminaUpdate)
          (Variables|/Script/Engine.CharacterMovementComponent|SetMaxWalkSpeed _charactermovement 5e+02)))))
  (:Completed
    (goto _label)))

(event Input|EnhancedActionEvents|EnhancedInputActionIA_Space
  (params (ActionValue :type Boolean) (ElapsedSeconds :type Float%20%28double-precision%29) (TriggeredSeconds :type Float%20%28double-precision%29) (InputAction :type Input%20Action%20Object%20Reference :default "/Game/01_BluePrint/00_Global/Input/IA_Space.IA_Space"))
  ;[1 1 1] 스페이스바 - 굴러서 회피
  (:Started
    (if (not (or (Variables|체력|GetIsDie) (Variables|공격|GetIsAttack)))
      (if (not (Variables|회피|GetIsRoll))
        (Variables|회피|SetIsRoll true)
        (bind (_roll _curst) (CallFunction|UseRollST))
        (if _roll
          (Variables|스테미나|SetCurST _curst)
          (Animation|Montage|PlayMontage (Variables|Character|GetMesh) "/Game/02_Resource/Anim/Paladin/AM_Paladin_Roll.AM_Paladin_Roll"
            (:then
              _))
          (else
            (Variables|스테미나|SetCurST (+ _curst (Variables|스테미나|GetRollST)))
            (CallFunction|ResetRoll)))
        (CallFunction|SteminaUpdate)))))

(event Input|EnhancedActionEvents|EnhancedInputActionIA_MouseRightClick
  (params (ActionValue :type Boolean) (ElapsedSeconds :type Float%20%28double-precision%29) (TriggeredSeconds :type Float%20%28double-precision%29) (InputAction :type Input%20Action%20Object%20Reference :default "/Game/01_BluePrint/00_Global/Input/IA_MouseRightClick.IA_MouseRightClick"))
  (bind _mesh (Variables|Character|GetMesh))
  ;[1 1 1] 마우스 오른쪽 클릭 - 방어
  (:Triggered
    (if (Variables|Default|GetIsBlock)
      (Animation|Montage|PlayMontage _mesh "/Game/02_Resource/Anim/Paladin/AM_Paladin_Block_Idle.AM_Paladin_Block_Idle"
        (:then
          (bind _useblockingst (Timeline|타임라인_UseBlockingST Play)
            (:Update
              (Variables|스테미나|SetCurST (- (Variables|스테미나|GetCurST) _useblockingst))
              (CallFunction|SteminaUpdate)))))))
  (:Started
    (if (not (Math|Boolean|ORBoolean (Variables|공격|GetIsAttack) (Variables|체력|GetIsDie) (Variables|회피|GetIsRoll)))
      (if (Variables|Default|GetIsBlock)
        (Animation|Montage|PlayMontage _mesh "/Game/02_Resource/Anim/Paladin/AM_Paladin_Block_Start.AM_Paladin_Block_Start")
        (else
          (Variables|Default|SetIsBlock true)))))
  (:Completed
    (if (Variables|Default|GetIsBlock)
      (Variables|Default|SetIsBlock false)
      (Animation|Montage|PlayMontage _mesh "/Game/02_Resource/Anim/Paladin/AM_Paladin_Block_End.AM_Paladin_Block_End" 2.0
        (:then
          (CallFunction|SteminaUpdate))))))

(event EventBeginPlay)

(event Collision|EventActorBeginOverlap
  (params (OtherActor :type Actor%20Object%20Reference)))

(event EventTick
  (params (DeltaSeconds :type Float%20%28single-precision%29))
  (bind _asabp_paladin (Utilities|Casting|CastToABP_Paladin (Components|SkeletalMesh|GetAnimInstance (Variables|Character|GetMesh))))
  (if (Math|Boolean|ORBoolean (Variables|/Game/01_BluePrint/01_Character/ABP_Paladin.ABP_Paladin_C|GetIsShiftDown _asabp_paladin) (Variables|공격|GetIsAttack) (Variables|공격|GetIsComboAttack) (Variables|회피|GetIsRoll) (Variables|Default|GetIsBlock))
    (bind _recorverytime (Timeline|타임라인_RecorveryST SetNewTime)
      (:Update
        (CallFunction|RecorveryST _recorverytime)
        (CallFunction|SteminaUpdate)))
    (else
      (Timeline|타임라인_RecorveryST Play))))

(event Game|Damage|EventAnyDamage
  (params (Damage :type Float%20%28single-precision%29) (DamageType :type Damage%20Type%20Object%20Reference) (InstigatedBy :type Controller%20Object%20Reference) (DamageCauser :type Actor%20Object%20Reference))
  (if (Variables|회피|GetIsRoll)
    (CallFunction|HPUpdate)
    (else
      (if (Variables|Default|GetIsBlock)
        (CallFunction|ShieldSound)
        (bind _output_get (Variables|몬스터|SetMonsterDamege Damage))
        (if (<= (- _output_get (Variables|Default|GetBlockDamege)) 0.0)
          (bind _output_get_2 (Variables|몬스터|SetMonsterDamege 0.0))
          (Variables|체력|SetCurHP (- (Variables|체력|GetCurHP) _output_get_2))
          (else
            (bind _output_get_3 (Variables|몬스터|SetMonsterDamege (- _output_get (Variables|Default|GetBlockDamege))))
            (Variables|체력|SetCurHP (- (Variables|체력|GetCurHP) _output_get_3))))
        (else
          (bind _output_get_4 (Variables|몬스터|SetMonsterDamege Damage))
          (Variables|체력|SetCurHP (- (Variables|체력|GetCurHP) _output_get_4))))
      (CallFunction|HPUpdate))))

(event Input|KeyboardEvents|NumPadOne
  (params (Key :type Key%20Structure :default "None"))
  ;[1 1 1] 넘버락 1번키 - 플레이어 체력 MAX 치트키
  (:Pressed
    (if (not (Variables|체력|GetIsDie))
      (Variables|체력|SetCurHP (Variables|체력|GetmaxHP))
      (CallFunction|HPUpdate))))

(fn ConstructionScript)

(fn AttackSpentST
  (bind _attackst (Variables|스테미나|GetAttackST))
  (bind _curst (Variables|스테미나|GetCurST))
  (bind _returnvalue (- _curst _attackst))
  (return (>= _returnvalue 0.0) _returnvalue))

(fn UseRollST
  (bind _curst (Variables|스테미나|GetCurST))
  (bind _rollst (Variables|스테미나|GetRollST))
  (bind _returnvalue (- _curst _rollst))
  (return (>= _returnvalue 0.0) _returnvalue))

(fn RecorveryST
  (params (deltaTime :type Float%20%28double-precision%29))
  (if (<= (Variables|스테미나|GetCurST) (Variables|스테미나|GetMaxST))
    (Variables|스테미나|SetCurST (+ (Variables|스테미나|GetCurST) deltaTime))
    (else
      (Variables|스테미나|SetCurST (Variables|스테미나|GetMaxST)))))